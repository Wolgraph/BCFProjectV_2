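; Editor-side manager actor for loading saved Collaborative Viewer states outside of play.
; BeginPlayEditor tags actors by name with a CollabName_ prefix, then starts the SaveLoadStateController with the persistent UI and save/load pawn.
; It then flags each BP_BaseCommandComponent as running from the editor, initializes it and binds it to the save game.
; Remove destroys those components and the actor, and also runs on BeginPlay so the manager never persists into play.
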(event `Remove`
  (for _array_element (`self.K2_GetComponentsByClass` "/Game/CollaborativeViewer/Blueprints/Commands/BP_BaseCommandComponent.BP_BaseCommandComponent_C")
    (`/Game/CollaborativeViewer/Blueprints/Commands/BP_BaseCommandComponent.DestroyInEditor` _array_element))
  (`self.K2_DestroyActor`))

(event `self.ReceiveBeginPlay`
  (`self.Remove`))

(event `BeginPlayEditor`
  (params (Persistent_UI :type "/Game/CollaborativeViewer/UMG/GameMenu/Persistent_ToolBar Object Reference"))
  (bind _outactors (`GameplayStatics.GetAllActorsOfClass` "/Script/Engine.Actor"))
  (bind _interactive_actors (`/Game/CollaborativeViewer/Blueprints/ShareLibrary/CommonFunctions_CV.Add Actor Name as Tag` _outactors))
  (set `self.Interactive Actors` _interactive_actors)
  (`/Game/CollaborativeViewer/Blueprints/SaveGame/SaveLoad_State_Controller.BeginPlayFromEditor` (`self.SaveLoad_State_Controller`) Persistent_UI (`self.SaveLoad_State_Pawn`))
  (for _array_element (`self.K2_GetComponentsByClass` "/Game/CollaborativeViewer/Blueprints/Commands/BP_BaseCommandComponent.BP_BaseCommandComponent_C")
    (bind _asbp_base_command_component (cast `/Game/CollaborativeViewer/Blueprints/Commands/BP_BaseCommandComponent` _array_element))
    (set `/Game/CollaborativeViewer/Blueprints/Commands/BP_BaseCommandComponent.FromEditor` true _asbp_base_command_component)
    (`/Game/CollaborativeViewer/Blueprints/Commands/BP_BaseCommandComponent.BeginPLayEditor` _asbp_base_command_component)
    (`/Game/CollaborativeViewer/Blueprints/Commands/BP_BaseCommandComponent.BindSaveGame` _asbp_base_command_component Persistent_UI)))

(fn `UserConstructionScript`)