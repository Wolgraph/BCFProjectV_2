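; Collaborative Viewer command component that gives players with the Reviser role an "Issue" contextual button for saving the project's BCF topics.
; After pawn spawn it builds the button and binds its "Save Project" option to SaveProjects.
; SaveProjects compiles the PlayerController's project and version data into BCF files under OutputFiles.
; It then saves each topic's markup, viewpoint and snapshot, keyed by topic GUID.
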(event `self.ExecuteAfterSpawnPawn`
  (`parent.ExecuteAfterSpawnPawn`)
  (switch `/Game/CollaborativeViewer/Blueprints/PlayerController/PV_PlayingRoles` (`/Game/CollaborativeViewer/Blueprints/PlayerController/BP_Collab_V_PlayerController.Player Role` (cast `/Game/CollaborativeViewer/Blueprints/PlayerController/BP_Collab_V_PlayerController` (`GameplayStatics.GetPlayerController` 0) :!pure true))
    (:`NewEnumerator6`
      (set `self.Icon` "/Game/CollaborativeViewer/Blueprints/Commands/CreateTopic/IconTopic.IconTopic")
      (set `self.OptionsButtonNames` (`|MakeArray` "Save Project" :!type "Text"))
      (set `self.Name` "Issue")
      (`self.CreateContextualButon`)
      (`self.Bind Options`)
      (`self.BindSaveGame` (`self.Persistent UI`)))))

(event `Bind Options`
  (bind _asoption_button (cast `/Game/CollaborativeViewer/UMG/GameMenu/Option_Button` (`|GetArrayItem` (`self.OptionsButtons`)) :!pure true))
  (`|ExecutionSequence`
    (:`then_0`
      (set `/Game/CollaborativeViewer/UMG/GameMenu/Option_Button.WhenExecute` "NewEnumerator1" _asoption_button)
      (add `/Game/CollaborativeViewer/UMG/GameMenu/Option_Button.Execute` _asoption_button (delegate `Option_1`)))))

(event `Option_1`
  (params (id :type Integer) (Actor :type "Actor Object Reference") (IsRightHand :type Boolean))
  (`self.Save Projects`))

(event `Save Projects`
  (bind _returnvalue (`KismetStringLibrary.Concat_StrStr` (`BlueprintPathsLibrary.ProjectDir`) "OutputFiles/"))
  (bind _asbp_collab_v_player_controller (cast `/Game/CollaborativeViewer/Blueprints/PlayerController/BP_Collab_V_PlayerController` (`GameplayStatics.GetPlayerController` 0) :!pure true))
  (`|ExecutionSequence`
    (:`then_0`
      (bind _returnvalue_2 (`BCF_Parser.FCompileProjectFile` (`/Game/CollaborativeViewer/Blueprints/PlayerController/BP_Collab_V_PlayerController.ProjectFile` _asbp_collab_v_player_controller)))
      (`BCF_Parser.FSaveFile` _returnvalue_2 _returnvalue "project.bcfp"))
    (:`then_1`
      (bind _returnvalue_3 (`BCF_Parser.FCompileVersionFile` (`/Game/CollaborativeViewer/Blueprints/PlayerController/BP_Collab_V_PlayerController.VersionFile` _asbp_collab_v_player_controller)))
      (`BCF_Parser.FSaveFile` _returnvalue_3 _returnvalue "bcf.version" true))
    (:`then_2`
      (for _array_element (`/Game/CollaborativeViewer/Blueprints/PlayerController/BP_Collab_V_PlayerController.Topic list` _asbp_collab_v_player_controller)
        (`|ExecutionSequence`
          (:`then_0`
            (bind (_markupfile _visualizationfile) (break `BCFTopicFile` _array_element))
            (bind _returnvalue_4 (`BCF_Parser.FCompileMarkup` _markupfile))
            (bind (_guid _index) (`self.GetTopicGUIDAndIndex` _markupfile))
            (`BCF_Parser.FSaveTopic` _returnvalue_4 _returnvalue _guid "markup.bcf"))
          (:`then_1`
            (bind _returnvalue_5 (`BCF_Parser.FCompileVisualization` _visualizationfile (`/Game/CollaborativeViewer/Blueprints/PlayerController/BP_Collab_V_PlayerController.Perspective` _asbp_collab_v_player_controller)))
            (`BCF_Parser.FSaveTopic` _returnvalue_5 _returnvalue _guid "viewpoint.bcfv"))
          (:`then_2`
            (`BCF_Parser.FSaveSnapshot` _returnvalue _guid (`KismetStringLibrary.Concat_StrStr` "snapshot" (`KismetStringLibrary.Conv_IntToString` _index) ".png"))))))))