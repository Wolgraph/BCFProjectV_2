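; Collaborative Viewer "Topic" command that offers Take Snapshot to all roles and Save Project to Revisers.
; Enabling Take Snapshot spawns a BP_Photo frame at the camera, movable through the pawn's BP_TransformComponent; executing it captures outside VR.
; Disabling restores collision and field of view and removes the frame.
; Save Project writes the player controller's BCF project, version and per-topic markup, viewpoint and snapshot files to OutputFiles.
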(event `self.ExecuteAfterSpawnPawn`
  (bind _array (`|MakeArray` "Take Snapshot" :!type "Text"))
  ;[0 1 0.1488] BeginPlay
  (set `self.Icon` "/Game/CollaborativeViewer/Blueprints/Commands/Snapshot/IconTopic.IconTopic")
  (set `self.OptionsButtonNames` (select `/Game/CollaborativeViewer/Blueprints/PlayerController/PV_PlayingRoles` (`/Game/CollaborativeViewer/Blueprints/GameInstance/BP_CollaborativeViewer_GameInstance.PlayerRoles` (cast `/Game/CollaborativeViewer/Blueprints/GameInstance/BP_CollaborativeViewer_GameInstance` (`GameplayStatics.GetGameInstance`) :!pure true)) :`NewEnumerator0` _array :`NewEnumerator6` (`|MakeArray` "Take Snapshot" "Save Project" :!type "Text") :`NewEnumerator7` _array))
  (set `self.Name` "Topic")
  (`self.SetVariables`)
  (`self.CreateContextualButon`)
  (`self.Bind_Options`)
  (add `/Game/CollaborativeViewer/Blueprints/Pawn/BP_BasePawn.MouseLeftPressed` (`self.BasePawn`) (delegate `LeftMousePressed`)))

(event `LeftMousePressed`
  (params (Actor :type "Actor Object Reference") (RightHand :type Boolean))
  (bind _returnvalue (`Actor.GetComponentByClass` (`self.BasePawn`) "/Game/CollaborativeViewer/Blueprints/Commands/Transform/BP_TransformComponent.BP_TransformComponent_C"))
  ;[0 1 0.1488] BeginPlay
  ;;[1 1 1] Binding Button
  (if (`self.Activated`)
    (bind _returnvalue_2 (`GameplayStatics.GetActorOfClass` "/Game/CollaborativeViewer/Blueprints/Commands/Snapshot/BPs/BP_Photo.BP_Photo_C"))
    (`/Game/CollaborativeViewer/Blueprints/Commands/Transform/BP_TransformComponent.SetStartTransform` (`Actor.GetComponentByClass` (`self.BasePawn`) "/Game/CollaborativeViewer/Blueprints/Commands/Transform/BP_TransformComponent.BP_TransformComponent_C") _returnvalue_2 RightHand)
    (`/Game/CollaborativeViewer/Blueprints/Commands/Transform/BP_TransformComponent.SetupTransformComponent` _returnvalue false true false false)
    (`/Game/CollaborativeViewer/Blueprints/Commands/Transform/BP_TransformComponent.SetupTransformComponent` _returnvalue false true false false)
    (if RightHand
      (set `/Game/CollaborativeViewer/Blueprints/Commands/Transform/BP_TransformComponent.Is_R_Updating` true _returnvalue)
      (else
        (set `/Game/CollaborativeViewer/Blueprints/Commands/Transform/BP_TransformComponent.Is_L_Updating` true _returnvalue)))))

(event `Bind_Options`
  (bind _optionsbuttons (`self.OptionsButtons`))
  (bind _asoption_button (cast `/Game/CollaborativeViewer/UMG/GameMenu/Option_Button` (`|GetArrayItem` (`self.OptionsButtons`)) :!pure true))
  (bind _asoption_button_2 (cast `/Game/CollaborativeViewer/UMG/GameMenu/Option_Button` (`|GetArrayItem` _optionsbuttons 1) :!pure true))
  ;[0.3384 0.6313 1] Setup Option Buttons
  (`|ExecutionSequence`
    (:`then_0`
      (set `/Game/CollaborativeViewer/UMG/GameMenu/Option_Button.WhenExecute` "NewEnumerator0" _asoption_button)
      (add `/Game/CollaborativeViewer/UMG/GameMenu/Option_Button.Execute` _asoption_button (delegate `Option1`))
      (add `/Game/CollaborativeViewer/UMG/GameMenu/Option_Button.Enabled` _asoption_button (delegate `Enabled`))
      (add `/Game/CollaborativeViewer/UMG/GameMenu/Option_Button.Disabled` _asoption_button (delegate `OnDisable`))
      (add `Actor.OnDestroyed` (`GameplayStatics.GetPlayerPawn` 0) (delegate `OnDestroyed`)))
    (:`then_1`
      (if (> (`KismetArrayLibrary.Array_Length` _optionsbuttons) 1)
        (set `/Game/CollaborativeViewer/UMG/GameMenu/Option_Button.WhenExecute` "NewEnumerator1" _asoption_button_2)
        (add `/Game/CollaborativeViewer/UMG/GameMenu/Option_Button.Execute` _asoption_button_2 (delegate `Option2`))))))

(event `OnDestroyed`
  (params (DestroyedActor :type "Actor Object Reference"))
  ;[0.3384 0.6313 1] Setup Option Buttons
  (bind _returnvalue (`GameplayStatics.GetActorOfClass` "/Game/CollaborativeViewer/Blueprints/Commands/Snapshot/BPs/BP_Photo.BP_Photo_C" :!label _label))
  (`/Engine/EditorBlueprintResources/StandardMacros.IsValid` _returnvalue
    (:`Is Valid`
      (`Actor.K2_DestroyActor` _returnvalue))))

(event `Enabled`
  (bind _basepawn (`self.BasePawn`))
  ;[0.3384 0.6313 1] Setup Option Buttons
  (set `self.Activated` true)
  (set `/Game/CollaborativeViewer/Blueprints/Pawn/BP_BasePawn.CollisionType` (`|MakeArray` "ObjectTypeQuery9" :!type "EObjectTypeQuery Enum") _basepawn)
  (`/Engine/EditorBlueprintResources/StandardMacros.IsValid` _basepawn
    (:`Is Valid`
      (`self.Setup`))))

(event `OnDisable`
  (bind _returnvalue (`GameplayStatics.GetPlayerPawn` 0))
  (bind _basepawn (`self.BasePawn`))
  (bind _returnvalue_2 (`Actor.GetComponentByClass` _returnvalue "/Game/CollaborativeViewer/Blueprints/Commands/Transform/BP_TransformComponent.BP_TransformComponent_C"))
  ;[0.3384 0.6313 1] Setup Option Buttons
  (set `self.Activated` false)
  (set `/Game/CollaborativeViewer/Blueprints/Pawn/BP_BasePawn.CollisionType` (`|MakeArray` "ObjectTypeQuery1" "ObjectTypeQuery2" :!type "EObjectTypeQuery Enum") _basepawn)
  (set `CameraComponent.FieldOfView` 90.0 (`/Game/CollaborativeViewer/Blueprints/Pawn/BP_BasePawn.Camera` _basepawn))
  (`/Engine/EditorBlueprintResources/StandardMacros.IsValid` _returnvalue
    (:`Is Valid`
      (`/Game/CollaborativeViewer/Blueprints/Commands/Transform/BP_TransformComponent.SetupTransformComponent` _returnvalue_2 false false false false)
      (set `/Game/CollaborativeViewer/Blueprints/Commands/Transform/BP_TransformComponent.Is_L_Updating` false _returnvalue_2)
      (set `/Game/CollaborativeViewer/Blueprints/Commands/Transform/BP_TransformComponent.Is_R_Updating` false _returnvalue_2)
      (goto _label))))

(event `Option1`
  (params (id :type Integer) (Actor :type "Actor Object Reference") (IsRightHand :type Boolean))
  ;[0.3384 0.6313 1] Setup Option Buttons
  (if (not (`HeadMountedDisplayFunctionLibrary.IsHeadMountedDisplayEnabled`))
    (bind _returnvalue (`GameplayStatics.GetActorOfClass` "/Game/CollaborativeViewer/Blueprints/Commands/Snapshot/BPs/BP_Photo.BP_Photo_C"))
    (`/Game/CollaborativeViewer/Blueprints/Commands/Snapshot/BPs/BP_Photo.DoCapture` _returnvalue)))

(event `Option2`
  (params (id :type Integer) (Actor :type "Actor Object Reference") (IsRightHand :type Boolean))
  ;[0.3384 0.6313 1] Setup Option Buttons
  (`self.SaveProject`))

(event `Setup`
  (bind _returnvalue (`GameplayStatics.GetPlayerController` 0))
  (bind _basepawn (`self.BasePawn`))
  (bind (_returnvalue_location _returnvalue_rotation) (`KismetMathLibrary.BreakTransform` (`SceneComponent.K2_GetComponentToWorld` (`/Game/CollaborativeViewer/Blueprints/Pawn/BP_BasePawn.Camera` _basepawn))))
  ;[1 1 1] Set photo Frame Location
  (set `self.PhotoTransform` (`KismetMathLibrary.MakeTransform` _returnvalue_location _returnvalue_rotation (`KismetMathLibrary.Conv_DoubleToVector` (`/Game/CollaborativeViewer/Blueprints/Pawn/BP_BasePawn.CurrentWorldScale` _basepawn))))
  ;[1 1 1] Delete previous BP Photo
  (bind _outactors (`GameplayStatics.GetAllActorsOfClass` "/Game/CollaborativeViewer/Blueprints/Commands/Snapshot/BPs/BP_Photo.BP_Photo_C"))
  (`Actor.K2_DestroyActor` _outactors)
  ;[1 1 1] Create new BP Photo
  (bind _returnvalue_2 (`|SpawnActorFromClass` "/Game/CollaborativeViewer/Blueprints/Commands/Snapshot/BPs/BP_Photo.BP_Photo_C" (`self.PhotoTransform`) "Undefined" "OverrideRootScale" _returnvalue (`Controller.K2_GetPawn` _returnvalue)))
  (`/Game/CollaborativeViewer/Blueprints/Commands/Snapshot/BPs/BP_Photo.Init` _returnvalue_2))

(event `SaveProject`
  (bind _returnvalue (`KismetStringLibrary.Concat_StrStr` (`BlueprintPathsLibrary.ProjectDir`) "OutputFiles/"))
  (bind _asbp_collab_v_player_controller (cast `/Game/CollaborativeViewer/Blueprints/PlayerController/BP_Collab_V_PlayerController` (`GameplayStatics.GetPlayerController` 0) :!pure true))
  ;[1 1 1] Save Project
  (`|ExecutionSequence`
    (:`then_0`
      (bind _returnvalue_2 (`BCF_Parser.FCompileProjectFile` (`/Game/CollaborativeViewer/Blueprints/PlayerController/BP_Collab_V_PlayerController.ProjectFile` _asbp_collab_v_player_controller)))
      (`BCF_Parser.FSaveFile` _returnvalue_2 _returnvalue "project.bcfp"))
    (:`then_1`
      (bind _returnvalue_3 (`BCF_Parser.FCompileVersionFile` (`/Game/CollaborativeViewer/Blueprints/PlayerController/BP_Collab_V_PlayerController.VersionFile` _asbp_collab_v_player_controller)))
      (`BCF_Parser.FSaveFile` _returnvalue_3 _returnvalue "bcf.version" true))
    (:`then_2`
      (for _array_element (`/Game/CollaborativeViewer/Blueprints/PlayerController/BP_Collab_V_PlayerController.Topic list` _asbp_collab_v_player_controller)
        (`|ExecutionSequence`
          (:`then_0`
            (bind (_markupfile _visualizationfile) (break `BCFTopicFile` _array_element))
            (bind _returnvalue_4 (`BCF_Parser.FCompileMarkup` _markupfile))
            (bind (_guid _index) (`self.GetTopigGUIDAndIndex` _markupfile))
            (`BCF_Parser.FSaveTopic` _returnvalue_4 _returnvalue _guid "markup.bcf"))
          (:`then_1`
            (bind _returnvalue_5 (`BCF_Parser.FCompileVisualization` _visualizationfile (`/Game/CollaborativeViewer/Blueprints/PlayerController/BP_Collab_V_PlayerController.Perspective` _asbp_collab_v_player_controller)))
            (`BCF_Parser.FSaveTopic` _returnvalue_5 _returnvalue _guid "viewpoint.bcfv"))
          (:`then_2`
            (`BCF_Parser.FSaveSnapshot` _returnvalue _guid (`KismetStringLibrary.Concat_StrStr` "snapshot" (`KismetStringLibrary.Conv_IntToString` _index) ".png"))))))))

(fn `GetTopigGUIDAndIndex`
  (params (NewParam :type "BCFMarkupXMLFile Structure"))
  (returns (GUID :type String) (Index :type Integer))
  (bind (_topicguid _title _topictype _referencelink _description _priority _index) (break `BCFTopic` (`.topic` (break `BCFMarkupXMLFile` NewParam))))
  (return _topicguid _index))