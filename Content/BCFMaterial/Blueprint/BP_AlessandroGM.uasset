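; BP_AlessandroGM builds BCF (BIM Collaboration Format) project and version file data on BeginPlay, storing them in ProjectFile and VersionFile.
; CompileProject creates the project with a fresh ID from NewStringGuid, which inserts hyphens into a new GUID and lowercases it.
; CompileVersion fills the version data but crosses its inputs, feeding VersionId into DetailedVersion and vice versa.
; The graphs only assemble these structures and write nothing to disk.
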(event `self.ReceiveBeginPlay`
  ;[1 1 1] Compilazione File di progetto
  (bind _projectoutput (`self.CompileProject`))
  (set `self.ProjectFile` _projectoutput)
  (bind _versionoutput (`self.CompileVersion` "2.0" "2.0 KUBUS BV"))
  (set `self.VersionFile` _versionoutput))

(fn `CompileProject`
  (returns (ProjectOutput :type "BCFProjectXMLFile Structure"))
  (return (make `BCFProjectXMLFile` (make `BCFProject` (`self.NewStringGuid`) true))))

(fn `CompileVersion`
  (params (VersionId :type String) (DetailedVersion :type String))
  (returns (VersionOutput :type "BCFVersionXMLFile Structure"))
  (return (make `BCFVersionXMLFile` VersionId true DetailedVersion)))

(fn `NewStringGuid`
  (returns (NewGuid :type String))
  (locals (_Guid :type String))
  (for (_array_element _array_index) (`KismetStringLibrary.GetCharacterArrayFromString` (`KismetGuidLibrary.Conv_GuidToString` (`KismetGuidLibrary.NewGuid`)))
    (if (or (== _array_index 8) (== _array_index 12) (== _array_index 16) (== _array_index 20))
      (set `local._Guid` (`KismetStringLibrary.Concat_StrStr` (`local._Guid`) "-" _array_element))
      (else
        (set `local._Guid` (`KismetStringLibrary.Concat_StrStr` (`local._Guid`) _array_element)))))
  (return (`KismetStringLibrary.ToLower` (`local._Guid`))))

(fn `UserConstructionScript`)