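; Player pawn for first-person navigation with snapshot capture for a topic form, apparently for BCF issue reporting.
; BeginPlay shows the main widget and creates the topic form; move and look axes only respond while that form is hidden.
; Takesnapshot captures the scene via SceneCapture2D, stores actor location plus camera forward, up and FOV in BP_AlessandroGM, then opens the form.
; A debug camera printout is left disconnected.
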(event `InputAxis|LookRight`
  (params (AxisValue :type "Float (single-precision)"))
  ;[1 1 1] Rotation
  (if (not (`Widget.IsVisible` (`self.Widget_Ref`)))
    (`self.AddControllerYawInput` AxisValue)))

(event `InputAxis|MoveForward` :consume false :overrideparent false
  (params (AxisValue :type "Float (single-precision)"))
  ;[1 1 1] Movement
  (if (not (`Widget.IsVisible` (`self.Widget_Ref`)))
    (`self.AddMovementInput` (`self.GetActorForwardVector`) AxisValue)))

(event `Take snapshot`
  (bind _cc_camera (`self.CC_Camera`))
  (`|ExecutionSequence`
    (:`then_0`
      (`SceneCaptureComponent2D.CaptureScene` (`self.SceneCaptureComponent2D`)))
    (:`then_1`
      (bind _asbp_alessandro_gm (cast `/Game/BCFMaterial/Blueprint/BP_AlessandroGM` (`GameplayStatics.GetGameMode`))))
    (:`then_2`
      (set `/Game/BCFMaterial/Blueprint/BP_AlessandroGM.CameraPosition` (`self.K2_GetActorLocation`) _asbp_alessandro_gm))
    (:`then_3`
      (set `/Game/BCFMaterial/Blueprint/BP_AlessandroGM.CameraDirection` (`SceneComponent.GetForwardVector` _cc_camera) _asbp_alessandro_gm))
    (:`then_4`
      (set `/Game/BCFMaterial/Blueprint/BP_AlessandroGM.CameraUpVector` (`SceneComponent.GetUpVector` _cc_camera) _asbp_alessandro_gm))
    (:`then_5`
      (set `/Game/BCFMaterial/Blueprint/BP_AlessandroGM.FieldOfView` (`CameraComponent.FieldOfView` _cc_camera) _asbp_alessandro_gm))
    (:`then_6`
      (`UserWidget.AddToViewport` (`self.Widget_Ref`) 1))))

(event `InputAxis|LookUp`
  (params (AxisValue :type "Float (single-precision)"))
  ;[1 1 1] Rotation
  (if (not (`Widget.IsVisible` (`self.Widget_Ref`)))
    (`self.AddControllerPitchInput` AxisValue)))

(event `InputAxis|MoveRight` :consume false :overrideparent false
  (params (AxisValue :type "Float (single-precision)"))
  ;[1 1 1] Movement
  (if (not (`Widget.IsVisible` (`self.Widget_Ref`)))
    (`self.AddMovementInput` (`self.GetActorRightVector`) AxisValue)))

(event `self.ReceiveTick`
  (params (DeltaSeconds :type "Float (single-precision)")))

(event `self.ReceiveBeginPlay`
  (bind _returnvalue (`GameplayStatics.GetPlayerController` 0))
  (set `self.GameManager` (cast `/Game/BCFMaterial/Blueprint/BP_AlessandroGM` (`GameplayStatics.GetGameMode`) :!pure true))
  (bind _returnvalue_2 (`|CreateWidget` "/Game/BCFMaterial/Blueprint/W_TopicForm.W_TopicForm_C" _returnvalue))
  (set `self.Widget_Ref` _returnvalue_2)
  (bind _returnvalue_3 (`|CreateWidget` "/Game/BCFMaterial/Blueprint/W_MainWidget.W_MainWidget_C" _returnvalue))
  (`UserWidget.AddToViewport` _returnvalue_3 0))

(fn `UserConstructionScript`)